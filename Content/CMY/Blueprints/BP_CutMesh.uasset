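; BP_CutMesh is a sliceable mesh actor that can be cut in two along a given plane at runtime.
; The construction script copies MeshVar into a procedural mesh with collision, then destroys the static mesh component.
; CustomEvent_0 slices that mesh, capping the cut with Cut_Material in a new section.
; The newly created half gets physics simulation and a fixed velocity-change impulse to launch it away.
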(event Custom|CustomEvent_0
  (params (PlanePosition :type Vector) (PlaneNormal :type Vector))
  (bind _outotherhalfprocmesh (Class|KismetProceduralMeshLibrary|SliceProceduralMesh (Variables|Default|GetProceduralMesh) PlanePosition PlaneNormal true "CreateNewSectionForCap" "/Game/CMY/Materials/Cut_Material.Cut_Material"))
  (Physics|SetSimulatePhysics _outotherhalfprocmesh true)
  (Physics|AddImpulse _outotherhalfprocmesh "1000.000000,1000.000000,1000.000000" "None" true))

(event EventBeginPlay)

(event Collision|EventActorBeginOverlap
  (params (OtherActor :type Actor%20Object%20Reference)))

(event EventTick
  (params (DeltaSeconds :type Float%20%28single-precision%29)))

(fn ConstructionScript
  (bind _staticmesh (Variables|Default|GetStaticMesh))
  (Components|StaticMesh|SetStaticMesh (Variables|Default|GetStaticMesh) (Variables|Default|GetMeshVar))
  (Class|KismetProceduralMeshLibrary|CopyProceduralMeshfromStaticMeshComponent _staticmesh 0 (Variables|Default|GetProceduralMesh) true)
  (Components|DestroyComponent _staticmesh))